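; Tower is a world actor that plays a whoosh sound while a Hovercraft is inside its Area trigger.
; Overlap begin and end events activate and deactivate the Whoosh component for Hovercraft actors only.
; While Whoosh is active, Tick scales its volume with the speed of player 0's pawn, capped at full volume, regardless of which Hovercraft triggered it.
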(event `self.ReceiveBeginPlay`)

(event `self.ReceiveActorBeginOverlap`
  (params (OtherActor :type "Actor Object Reference")))

(event `self.Area.OnComponentBeginOverlap`
  (params (OtherActor :type "Actor Object Reference") (OtherComp :type "PrimitiveComponent Object Reference") (OtherBodyIndex :type Integer) (bFromSweep :type Boolean) (SweepResult :type "HitResult Structure (by ref)"))
  (cast `/Game/Blueprints/Vehicles/Hovercraft` OtherActor)
  (`ActorComponent.Activate` (`self.Whoosh`) false))

(event `self.Area.OnComponentEndOverlap`
  (params (OtherActor :type "Actor Object Reference") (OtherComp :type "PrimitiveComponent Object Reference") (OtherBodyIndex :type Integer))
  (cast `/Game/Blueprints/Vehicles/Hovercraft` OtherActor)
  (`ActorComponent.Deactivate` (`self.Whoosh`)))

(event `self.ReceiveTick`
  (params (DeltaSeconds :type "Float (single-precision)"))
  (if (`ActorComponent.IsActive` (`self.Whoosh`))
    (`AudioComponent.SetVolumeMultiplier` (`self.Whoosh`) (`KismetMathLibrary.FMin` (/ (`KismetMathLibrary.VSize` (`self.GetVelocity` (`GameplayStatics.GetPlayerPawn` 0))) 15000.0) 1.0))))

(fn `UserConstructionScript`)