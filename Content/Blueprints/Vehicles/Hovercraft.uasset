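; Player-controlled physics hovercraft with thrust, steering, braking and a timed spool-up boost, updated every tick.
; Hoverpad child components trace to the surface and apply spring and damping forces scaled by distance and normal alignment.
; The fraction of grounded pads sets how strongly velocity swings toward the nose, while inputs add pitch and yaw torque.
; Speed drives engine audio; throttle and boost drive the flame material.
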(event EventBeginPlay)

(event Collision|EventActorBeginOverlap
  (params (OtherActor :type Actor%20Object%20Reference)))

(event EventTick
  (params (DeltaSeconds :type Float%20%28single-precision%29))
  (Variables|Default|Setdt DeltaSeconds)
  (|Thrust
    (:%20
      (|Gravitation
        (:%20
          (|DirectionalControl
            (:%20
              (|VectorTrails
                (:%20
                  (|HandleControls
                    (:%20
                      (|Accelerating
                        (:%20
                          (|Braking
                            (:%20
                              (|Boosting))))))))))))))))

(event Input|ActionEvents|InputActionBoost
  (:Pressed
    (Variables|Default|SetBoostHeld true))
  (:Released
    (Variables|Default|SetBoostHeld false)))

(event Input|AxisEvents|InputAxisPullUp
  (params (AxisValue :type Float%20%28single-precision%29))
  (Variables|Default|SetControlPitch AxisValue))

(event Input|AxisEvents|InputAxisTurnRight
  (params (AxisValue :type Float%20%28single-precision%29))
  (Variables|Default|SetControlYaw AxisValue))

(event Input|AxisEvents|InputAxisAccelerate
  (params (AxisValue :type Float%20%28single-precision%29))
  (Variables|Default|SetAcceleration AxisValue))

(event Input|AxisEvents|InputAxisBrake
  (params (AxisValue :type Float%20%28single-precision%29))
  (Variables|Default|SetBrake AxisValue))

(fn ConstructionScript
  (bind _returnvalue (Rendering|Material|CreateDynamicMaterialInstance (Variables|Default|Gethover_flames) 0 0 :!class /Script/Engine.PrimitiveComponent))
  (Variables|Default|SetFlameMaterial _returnvalue))

(fn Gravpads
  (params (PhysObj :type Primitive%20Component%20Object%20Reference) (Strength :type Float%20%28single-precision%29))
  (Utilities|FlowControl|Sequence
    (:then_0
      (LocalVariables|SetPhysics%20Object PhysObj))
    (:then_1
      (LocalVariables|SetGravStrength Strength)
      (Variables|Default|SetGravEngaged 0.0)
      (LocalVariables|SetGravPadsTotal 0.0))
    (:then_2
      ;[1 1 1] Cycle through the hoverpads and determine their grav vectors
      (for _array_element (Components|GetChildrenComponents (LocalVariables|GetPhysics%20Object) true)
        (bind _ashoverpad (Utilities|Casting|CastToHoverpad _array_element))
        (Utilities|FlowControl|Sequence
          (:then_0
            (bind _output_get (LocalVariables|SetGravOrigin (Transformation|GetWorldLocation _ashoverpad)))
            (bind _output_get_2 (LocalVariables|SetGravVector (Math|Vector|RotateVector (Variables|/Game/Blueprints/Vehicles/Hoverpad.Hoverpad_C|GetGravVector _ashoverpad) (Transformation|GetWorldRotation _ashoverpad))))
            (LocalVariables|SetGravCenter (+ _output_get _output_get_2)))
          (:then_1
            (LocalVariables|SetVelocityVector (- (Transformation|GetWorldLocation _ashoverpad) (Variables|/Game/Blueprints/Vehicles/Hoverpad.Hoverpad_C|GetLastPosition _ashoverpad)))
            (Variables|/Game/Blueprints/Vehicles/Hoverpad.Hoverpad_C|SetLastPosition _ashoverpad (Transformation|GetWorldLocation _ashoverpad)))
          (:then_2
            (LocalVariables|SetGravPadsTotal (+ (LocalVariables|GetGravPadsTotal) 1.0)))
          (:then_3
            ;[1 1 1] Trace to ground and collect values
            (bind (_outhit _returnvalue) (Collision|LineTraceByChannel (LocalVariables|GetGravOrigin) (+ (LocalVariables|GetGravOrigin) (LocalVariables|GetGravVector) (LocalVariables|GetGravVector)) "TraceTypeQuery3" true 0 "None"))
            (Utilities|FlowControl|Sequence
              (:then_0
                (bind _output_get_3 (LocalVariables|SetHitLocation (.location _outhit)))
                (if _returnvalue
                  _))
              (:then_1
                (bind _output_get_4 (LocalVariables|SetGravInRange _returnvalue))
                (if _output_get_4
                  (LocalVariables|SetGravToSurfaceVector (- _output_get_3 (LocalVariables|GetGravOrigin)))
                  (Variables|Default|SetGravEngaged (+ (Variables|Default|GetGravEngaged) 1.0))))
              (:then_2
                (LocalVariables|SetHitNormal (.normal _outhit)))
              (:then_3
                ;[1 1 1] Skip if not in grav range.
                (if (LocalVariables|GetGravInRange)
                  (Utilities|FlowControl|Sequence
                    (:then_0
                      (Class|PrimitiveComponent|AddForceatLocation (LocalVariables|GetPhysics%20Object) (* (* (- (LocalVariables|GetGravToSurfaceVector) (LocalVariables|GetGravVector)) (* (LocalVariables|GetGravStrength) 2e+02)) (* (- (* (Math|Vector|DotProduct (LocalVariables|GetHitNormal) (Math|Vector|Normalize (LocalVariables|GetGravVector))) -2.0) 1.0) (Math|Float|Clamp(Float) (/ (- (* (Math|Vector|VectorLength (LocalVariables|GetGravVector)) 2.0) (Math|Vector|VectorLength (LocalVariables|GetGravToSurfaceVector))) (* (Math|Vector|VectorLength (LocalVariables|GetGravVector)) 2.0))))) (LocalVariables|GetGravOrigin) "None"))
                    (:then_1
                      (bind _v (CallFunction|Projection (LocalVariables|GetVelocityVector) (LocalVariables|GetGravVector)))
                      (Class|PrimitiveComponent|AddForceatLocation (LocalVariables|GetPhysics%20Object) (* (* (Math|Vector|NegateVector _v) (* (LocalVariables|GetGravStrength) 2.5e+02)) (* (- (* (Math|Vector|DotProduct (LocalVariables|GetHitNormal) (Math|Vector|Normalize (LocalVariables|GetGravVector))) -2.0) 1.0) (Math|Float|Clamp(Float) (/ (- (* (Math|Vector|VectorLength (LocalVariables|GetGravVector)) 2.0) (Math|Vector|VectorLength (LocalVariables|GetGravToSurfaceVector))) (* (Math|Vector|VectorLength (LocalVariables|GetGravVector)) 2.0))))) (LocalVariables|GetGravOrigin) "None"))))))))))
    (:then_3
      (Variables|Default|SetGravEngaged (/ (Variables|Default|GetGravEngaged) (LocalVariables|GetGravPadsTotal))))))

(fn BoostSpooled
  (Variables|Default|SetBoostMult 2.2)
  (Variables|Default|SetBoostActive true))

(fn Projection
  (params (A :type Vector) (B :type Vector))
  (bind (_x _y _z) (Math|Vector|BreakVector B))
  (bind (_x_2 _y_2 _z_2) (Math|Vector|BreakVector A))
  (bind (_x_3 _y_3 _z_3) (Math|Vector|BreakVector B))
  (Utilities|FlowControl|Sequence
    (:then_0
      (LocalVariables|Setdp (+ (* _x_2 _x_3) (* _y_2 _y_3) (* _z_2 _z_3))))
    (:then_1
      (LocalVariables|Setdsq (+ (Math|Float|Square _x) (Math|Float|Square _y) (Math|Float|Square _z))))
    (:then_2
      (return (* B (/ (LocalVariables|Getdp) (LocalVariables|Getdsq)))))))